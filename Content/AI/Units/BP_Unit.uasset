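; Base AI unit character that carries a socket-attached weapon, exposes team, attack range and movement tag, and manages health and walk speed.
; Attacks fire the weapon only while health remains.
; On death it ragdolls, stops firing and, for Neutral or Hostile teams, passes its data-table cost to the player state's money update.
; SetupMesh is empty, and a team-color darkening chain is left unconnected.
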(event Custom|OnKilled
  (bind _mesh (Variables|Character|GetMesh))
  (Collision|SetCollisionEnabled (Variables|Collision|GetCapsuleComponent) "NoCollision")
  (Collision|SetCollisionProfileName _mesh "Ragdoll" true :!class /Script/Engine.PrimitiveComponent)
  (Physics|SetSimulatePhysics _mesh true)
  (CallFunction|StopAttack)
  (Actor|SetLifeSpan self 0.0)
  (switch Utilities|FlowControl|Switch|SwitchonETeamAttitude (Variables|Default|GetTeamId)
    (:Neutral
      _)
    (:Hostile
      _))
  (bind _out_row (Utilities|GetUnitInfoDataTable (Variables|Default|GetRow%20Name))
    (:Row%20Found
      (Default|UpdateMoney (CallFunction|GetPlayerStateBP) (.Cost (Utilities|Struct|BreakST_UnitInfo _out_row))))))

(event Custom|InitializeHealth
  (params (DefaultHealth :type Integer))
  (Default|InitializeHealth (Variables|Default|GetHealthComponent) DefaultHealth))

(event EventBeginPlay
  (EventDispatchers|BindEventtoOnKilled (Variables|Default|GetHealthComponent) (delegate Custom|OnKilled)))

(event EventAttack
  (bind _weapon (Variables|Default|GetWeapon))
  (Math|Integer|CompareInt (Default|GetHealth (Variables|Default|GetHealthComponent))
    (:>
      (Utilities|IsValid _weapon
        (:Is%20Valid
          (Default|FireWeapon _weapon))))))

(event EventStopAttack
  (bind _weapon (Variables|Default|GetWeapon))
  (Utilities|IsValid _weapon
    (:Is%20Valid
      (Default|StopFiring _weapon))))

(fn ConstructionScript)

(fn SetupMesh)

(fn SpawnWeapon
  (params (Row%20Name :type Name) (WeaponClass :type BP%20Weapon%20Class%20Reference))
  (bind _self self)
  (bind _output_get (Variables|Default|SetRow%20Name Row%20Name))
  (bind _returnvalue (Game|SpawnActorfromClass WeaponClass (Math|Transform|MakeTransform "0, 0, 0" "0, 0, 0" "1.000000,1.000000,1.000000") "AdjustIfPossibleButAlwaysSpawn" _self _output_get _self))
  (bind _output_get_2 (Variables|Default|SetWeapon _returnvalue))
  (Transformation|AttachComponentToComponent _output_get_2 (Variables|Character|GetMesh) "Socket_Weapon" "SnapToTarget" "SnapToTarget" "SnapToTarget" true))

(fn InitializeWalkSpeed
  (params (Max%20Walk%20Speed :type Float%20%28single-precision%29))
  (CallFunction|SetWalkSpeed Max%20Walk%20Speed)
  (Variables|Default|SetDefaultWalkSpeed (Variables|/Script/Engine.CharacterMovementComponent|GetMaxWalkSpeed (Variables|Character|GetCharacterMovement))))

(fn SetWalkSpeed
  (params (Max%20Walk%20Speed :type Float%20%28single-precision%29))
  (Variables|/Script/Engine.CharacterMovementComponent|SetMaxWalkSpeed (Variables|Character|GetCharacterMovement) Max%20Walk%20Speed))

(fn GetAttackRange
  (return (Variables|Default|GetAttackRange)))

(fn GetMovementTag
  (return (Variables|Default|GetMovementTag)))

(fn GetTeamId
  (return (Variables|Default|GetTeamId)))