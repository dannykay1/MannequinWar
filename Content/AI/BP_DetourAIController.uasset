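; AI controller that picks attack targets through perception and shuts down when its pawn is killed.
; On possession it binds to the pawn's BPC_Health killed event, then on death stops movement and the brain component's logic.
; Perception updates pass through attackability and alive checks before writing the actor to the TargetActor blackboard key, which is never cleared here.
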(event OnTargetPerceptionUpdated(AIPerception)
  (params (Actor :type Actor%20Object%20Reference) (Stimulus :type AI%20Stimulus%20Structure))
  (bind _blackboard (Variables|Default|GetBlackboard))
  (Utilities|CanAttackActor Actor (Pawn|GetControlledPawn)
    (:Yes
      (Utilities|IsActorAlive Actor
        (:Yes
          (Utilities|IsValid _blackboard
            (:Is%20Valid
              (AI|Components|Blackboard|SetValueasObject _blackboard (Utilities|Name|MakeLiteralName "TargetActor") Actor))))))))

(event Custom|OnControlledPawnKilled
  (bind _braincomponent (Variables|Default|GetBrainComponent))
  (AI|Navigation|StopMovement)
  (Utilities|IsValid _braincomponent
    (:Is%20Valid
      (AI|Logic|StopLogic _braincomponent "Killed"))))

(event EventPossess
  (params (PossessedPawn :type Pawn%20Object%20Reference))
  (bind _returnvalue (Pawn|GetControlledPawn))
  (bind _returnvalue_2 (Actor|GetComponentbyClass _returnvalue "/Game/Blueprints/Components/BPC_Health.BPC_Health_C"))
  (Utilities|IsValid _returnvalue_2
    (:Is%20Valid
      (EventDispatchers|BindEventtoOnKilled _returnvalue_2 (EventDispatchers|CreateEvent :!event Custom|OnControlledPawnKilled)))))

(fn ConstructionScript)