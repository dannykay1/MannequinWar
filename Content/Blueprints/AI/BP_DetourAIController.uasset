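; BP_DetourAIController is an AI controller that sends its controlled pawn wandering around the level's TargetPoints.
; On BeginPlay it sets focus once on a random BP_Unit, then enters an endless move loop.
; Each pass waits a short random delay, picks a random reachable point within a random radius of a random TargetPoint, and runs AIMoveTo with a loose acceptance radius, repeating on success or failure.
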(event EventBeginPlay
  (bind _outactors (Actor|GetAllActorsOfClass "/Game/Blueprints/AI/BP_Unit.BP_Unit_C"))
  (AI|SetFocus (.OutItem (Utilities|Array|Random _outactors)))
  (Utilities|FlowControl|Delay (Math|Random|RandomFloatinRange 1.0 3.0) :!label _label)
  (bind _outactors_2 (Actor|GetAllActorsOfClass "/Script/Engine.TargetPoint"))
  (AI|AIMoveTo (Pawn|GetControlledPawn) (.RandomLocation (AI|Navigation|GetRandomReachablePointinRadius (Transformation|GetActorLocation (.OutItem (Utilities|Array|Random _outactors_2))) (Math|Random|RandomFloatinRange 0.0 2e+03) 0 0)) 0 5e+02 false
    (:OnSuccess
      (goto _label))
    (:OnFail
      (goto _label))))

(fn ConstructionScript)