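; BP_Unit is an AI unit pawn whose weapon and appearance come from a unit data class.
; SetupUnit reads that class's defaults, then calls SpawnWeapon and SetupMesh.
; SpawnWeapon spawns the weapon owned by the unit and snaps it to the mesh's Socket_Weapon.
; SetupMesh swaps the skeletal mesh and creates a dynamic material per slot to apply the color through the Tint parameter.
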(event EventBeginPlay)

(fn ConstructionScript)

(fn SetupMesh
  (params (NewMesh :type Skeletal%20Mesh%20Object%20Reference) (MeshColor :type Linear%20Color%20Structure))
  (bind _mesh (Variables|Character|GetMesh))
  (Class|SkinnedMeshComponent|SetSkeletalMesh _mesh NewMesh true)
  (for (_array_element _array_index) (Rendering|Material|GetMaterials _mesh)
    (bind _returnvalue (Rendering|Material|CreateDynamicMaterialInstance _array_element "None" "None" :!class /Script/Engine.KismetMaterialLibrary))
    (Rendering|Material|SetMaterial (Variables|Character|GetMesh) _array_index _returnvalue)
    (Rendering|Material|SetVectorParameterValue _returnvalue "Tint" MeshColor :!class /Script/Engine.MaterialInstanceDynamic)))

(fn SetupUnit
  (params (UnitData :type DA%20Unit%20Info%20Class%20Reference))
  (bind (_weaponclass _mesh _meshcolor) (Utilities|GetClassDefaults UnitData))
  (CallFunction|SpawnWeapon _weaponclass)
  (CallFunction|SetupMesh _mesh _meshcolor))

(fn SpawnWeapon
  (params (WeaponClass :type Actor%20Class%20Reference))
  (bind _self self)
  (bind _returnvalue (Game|SpawnActorfromClass WeaponClass (Math|Transform|MakeTransform "0, 0, 0" "0, 0, 0" "1.000000,1.000000,1.000000") "AdjustIfPossibleButAlwaysSpawn" _self _self))
  (Transformation|AttachComponentToComponent _returnvalue (Variables|Character|GetMesh) "Socket_Weapon" "SnapToTarget" "SnapToTarget" "SnapToTarget" true))