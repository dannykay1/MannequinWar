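; Game mode that spawns team-based units and aims each one at another team's spawn point.
; Spawn points are added to a unique list through RegisterSpawnPoint.
; SpawnUnit looks up the unit's row in DT_UnitInfo and passes it to UnitCreator with a same-team spawn point and a different-team target point.
; Both point searches keep the last match in the list, so the target logic effectively suits two teams with one point each.
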(event Custom|SpawnUnit
  (params (UnitInfo :type Name))
  (bind _returnvalue (Utilities|GetDataTableRow "/Game/Data/DT_UnitInfo.DT_UnitInfo" UnitInfo)
    (:then
      (Default|CreateUnit (Variables|Default|GetUnitCreator) _returnvalue (CallFunction|FindSpawnPoint (.TeamId (Utilities|Struct|BreakST_UnitInfo _returnvalue))) (CallFunction|FindTargetPoint (.TeamId (Utilities|Struct|BreakST_UnitInfo _returnvalue)))))))

(event Custom|RegisterSpawnPoint
  (params (SpawnPoint :type BP%20Spawn%20Point%20Object%20Reference%20%28by%20ref%29))
  (Utilities|Array|AddUnique (Variables|Private|GetSpawnPoints) SpawnPoint))

(event EventBeginPlay)

(fn ConstructionScript)

(fn FindSpawnPoint
  (params (TeamID :type ETeamAttitude%20Enum :default "Friendly"))
  (for _array_element (Variables|Private|GetSpawnPoints)
    (if (Utilities|Enum|Equal(Enum) (Variables|/Game/Blueprints/BP_SpawnPoint.BP_SpawnPoint_C|GetTeamId _array_element) TeamID)
      (LocalVariables|SetLocalSpawnPoint _array_element)))
  (return (LocalVariables|GetLocalSpawnPoint)))

(fn FindTargetPoint
  (params (TeamID :type ETeamAttitude%20Enum :default "Friendly"))
  (for _array_element (Variables|Private|GetSpawnPoints)
    (if (Utilities|Enum|NotEqual(Enum) (Variables|/Game/Blueprints/BP_SpawnPoint.BP_SpawnPoint_C|GetTeamId _array_element) TeamID)
      (LocalVariables|SetLocalSpawnPoint _array_element)))
  (return (LocalVariables|GetLocalSpawnPoint)))