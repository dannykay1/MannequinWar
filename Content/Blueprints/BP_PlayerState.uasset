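; BP_PlayerState is a player state that tracks the player's money for buying units.
; It seeds the money pool from a starting amount on BeginPlay.
; UpdateMoney adds a signed amount, clamps the result to a fixed range and broadcasts OnMoneyUpdated with the new balance.
; CanSpawnUnit reports whether the pool covers a given cost.
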(event Custom|UpdateMoney
  (params (Amount :type Integer))
  (bind _output_get (Variables|Default|SetMoneyPool (Math|Integer|Clamp(Integer) (+ Amount (Variables|Default|GetMoneyPool)) 0 999999)))
  (Default|CallOnMoneyUpdated _output_get))

(event EventBeginPlay
  (Variables|Default|SetMoneyPool (Variables|Default|GetStartingMoney)))

(fn ConstructionScript)

(fn CanSpawnUnit
  (params (Cost :type Integer))
  (return (>= (- (Variables|Default|GetMoneyPool) Cost) 0)))