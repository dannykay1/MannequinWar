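; Health component that tracks its owning actor's integer health and signals changes and death.
; On BeginPlay it sets Health to DefaultHealth and binds to the owner's point and radial damage events.
; Each handler subtracts damage, clamps and truncates the result, then calls OnHealthChanged.
; At zero health it calls OnKilled through a separate DoOnce per damage type, so each path can fire it once.
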(event Custom|OnTakePointDamage
  (params (DamagedActor :type Actor%20Object%20Reference) (Damage :type Float%20%28single-precision%29) (InstigatedBy :type Controller%20Object%20Reference) (HitLocation :type Vector) (FHitComponent :type Primitive%20Component%20Object%20Reference) (BoneName :type Name) (ShotFromDirection :type Vector) (DamageType :type Damage%20Type%20Object%20Reference) (DamageCauser :type Actor%20Object%20Reference))
  (bind _output_get (Variables|Default|SetHealth (Math|Float|Truncate (Math|Float|Clamp(Float) (- (Variables|Default|GetHealth) Damage) 0.0 (Math|Conversions|ToFloat(Integer) (Variables|Default|GetHealth))))))
  (Default|CallOnHealthChanged)
  (Math|Integer|CompareInt _output_get
    (:==
      _)
    (:<
      _))
  (Utilities|FlowControl|DoOnce false
    (:Completed
      (Default|CallOnKilled))))

(event Custom|OnTakeRadialDamage
  (params (DamagedActor :type Actor%20Object%20Reference) (Damage :type Float%20%28single-precision%29) (DamageType :type Damage%20Type%20Object%20Reference) (Origin :type Vector) (HitInfo :type Hit%20Result%20Structure) (InstigatedBy :type Controller%20Object%20Reference) (DamageCauser :type Actor%20Object%20Reference))
  (bind _output_get (Variables|Default|SetHealth (Math|Float|Truncate (Math|Float|Clamp(Float) (- (Variables|Default|GetHealth) Damage) 0.0 (Math|Conversions|ToFloat(Integer) (Variables|Default|GetHealth))))))
  (Default|CallOnHealthChanged)
  (Math|Integer|CompareInt _output_get
    (:==
      _)
    (:<
      _))
  (Utilities|FlowControl|DoOnce false
    (:Completed
      (Default|CallOnKilled))))

(event EventBeginPlay
  (Variables|Default|SetHealth (Variables|Default|GetDefaultHealth))
  (EventDispatchers|BindEventtoOnTakePointDamage (Components|GetOwner) (EventDispatchers|CreateEvent :!event Custom|OnTakePointDamage))
  (EventDispatchers|BindEventtoOnTakeRadialDamage (Components|GetOwner) (EventDispatchers|CreateEvent :!event Custom|OnTakeRadialDamage)))