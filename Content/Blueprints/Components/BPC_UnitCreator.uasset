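; Actor component that spawns AI units from a unit info struct at a spawn point, facing a target point.
; CreateUnit validates both points, computes a yaw-only look-at transform, then SpawnUnit spawns the pawn class and applies health, weapon, team, movement tag and walk speed to the BP_Unit.
; After a short delay, it starts the BT_Unit behavior tree on the new unit's AI controller.
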(event Custom|CreateUnit
  (params (RowName :type Name) (UnitInfo :type ST%20Unit%20Config%20Structure) (SpawnPoint :type BP%20Spawn%20Point%20Object%20Reference) (TargetPoint :type BP%20Spawn%20Point%20Object%20Reference))
  (Utilities|AllObjectsValid? (Utilities|Array|MakeArray SpawnPoint TargetPoint)
    (:Is%20Valid
      (bind _spawnedunit (Private|SpawnUnit RowName UnitInfo (Private|CalculateSpawnTransform SpawnPoint TargetPoint)))
      (Utilities|FlowControl|Delay 0.2)
      (AI|RunBehaviorTree (AI|GetAIController _spawnedunit) "/Game/AI/BT_Unit.BT_Unit"))))

(fn SpawnUnit
  (params (RowName :type Name) (UnitInfo :type ST%20Unit%20Config%20Structure) (SpawnTransform :type Transform))
  (bind (_unitclass _cost _health _weaponclass _weapondamage _timebetweenshots _automaticfire_ _teamid _meshcolor _movementtag _walkspeed) (Utilities|Struct|BreakST_UnitConfig UnitInfo))
  (bind (_location _rotation) (Math|Transform|BreakTransform SpawnTransform))
  (bind _returnvalue (AI|SpawnAIFromClass _unitclass 0 _location _rotation false 0))
  (bind _asbp_unit (Utilities|Casting|CastToBP_Unit _returnvalue)
    (:then
      (Default|InitializeHealth _asbp_unit _health)
      (Default|SpawnWeapon _asbp_unit RowName _weaponclass)
      (Variables|/Game/AI/Units/BP_Unit.BP_Unit_C|SetTeamId _asbp_unit _teamid)
      (Variables|/Game/AI/Units/BP_Unit.BP_Unit_C|SetMovementTag _asbp_unit _movementtag)
      (Default|InitializeWalkSpeed _asbp_unit _walkspeed)
      (return _asbp_unit))
    (:CastFailed
      (return 0))))

(fn CalculateSpawnTransform
  (params (SpawnPoint :type BP%20Spawn%20Point%20Object%20Reference) (TargetPoint :type BP%20Spawn%20Point%20Object%20Reference))
  (return (Math|Transform|MakeTransform (Default|GetSpawnPoint SpawnPoint) (Math|Rotator|MakeRotator 0.0 0.0 (.yaw (Math|Rotator|FindLookatRotation (Transformation|GetActorLocation SpawnPoint) (Transformation|GetActorLocation TargetPoint)))) "1.000000,1.000000,1.000000")))