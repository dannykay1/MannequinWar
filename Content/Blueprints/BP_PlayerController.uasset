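; Player controller that turns player input into sideways movement and camera zoom for the controlled pawn.
; The MoveRight axis adds movement input along the fixed world Y axis.
; ZoomIn and ZoomOut send a negative or positive ZoomAmount through the BPI_CameraZoom interface, only if the pawn implements it.
; Unconnected leftover nodes hold an older zoom that edits the spring arm length directly with clamping.
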(event EventBeginPlay)

(event Input|ActionEvents|InputActionZoomIn
  (params (Key :type Key%20Structure :default "None"))
  (bind _returnvalue (Pawn|GetControlledPawn))
  (:Pressed
    (Utilities|DoesActorImplementInterface _returnvalue "/Game/Blueprints/Interfaces/BPI_CameraZoom.BPI_CameraZoom_C"
      (:Yes
        (Class|BPICameraZoom|Zoom(Message) _returnvalue (* (Variables|Default|GetZoomAmount) -1.0))))))

(event Input|ActionEvents|InputActionZoomOut
  (params (Key :type Key%20Structure :default "None"))
  (bind _returnvalue (Pawn|GetControlledPawn))
  (:Pressed
    (Utilities|DoesActorImplementInterface _returnvalue "/Game/Blueprints/Interfaces/BPI_CameraZoom.BPI_CameraZoom_C"
      (:Yes
        (Class|BPICameraZoom|Zoom(Message) _returnvalue (Variables|Default|GetZoomAmount))))))

(event Input|AxisEvents|InputAxisMoveRight
  (params (AxisValue :type Float%20%28single-precision%29))
  (Pawn|Input|AddMovementInput (Pawn|GetControlledPawn) "0.000000,1.000000, 0" AxisValue false))

(fn ConstructionScript)