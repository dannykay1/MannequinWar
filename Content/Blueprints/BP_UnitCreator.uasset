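; BP_UnitCreator spawns AI units from a UnitInfo struct at a given spawn point.
; CreateUnit adds SpawnOffset to the spawn point's location and passes it to SpawnUnit.
; SpawnUnit spawns the requested class with the BT_Unit behavior tree, casts it to BP_Unit, then applies weapon, team, mesh color, movement tag and speed from the struct.
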(event Custom|CreateUnit
  (params (UnitInfo :type ST%20Unit%20Info%20Structure) (SpawnPoint :type Actor%20Object%20Reference))
  (CallFunction|SpawnUnit UnitInfo (+ (Transformation|GetActorLocation SpawnPoint) (Variables|Default|GetSpawnOffset))))

(fn SpawnUnit
  (params (UnitInfo :type ST%20Unit%20Info%20Structure) (SpawnLocation :type Vector))
  (bind (_unitclass _weaponclass _teamid _meshcolor _movementtag _movementspeed) (Utilities|Struct|BreakST_UnitInfo UnitInfo))
  (bind _returnvalue (AI|SpawnAIFromClass _unitclass "/Game/AI/BT_Unit.BT_Unit" SpawnLocation "0, 0, 0" false 0))
  (bind _asbp_unit (Utilities|Casting|CastToBP_Unit _returnvalue))
  (Default|SpawnWeapon _asbp_unit _weaponclass)
  (Variables|/Game/AI/BP_Unit.BP_Unit_C|SetTeamId _asbp_unit _teamid)
  (Default|SetupMesh _asbp_unit _meshcolor)
  (Variables|/Game/AI/BP_Unit.BP_Unit_C|SetMovementTag _asbp_unit _movementtag)
  (Default|SetMovementSpeed _asbp_unit _movementspeed))