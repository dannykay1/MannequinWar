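; Projectile actor that deals fixed point damage to BP_Unit actors it overlaps, then destroys itself.
; Its Sphere has collision off at construction; BeginPlay makes it ignore the owner when moving, enables query-only collision and sets a limited lifespan.
; Unit overlaps and any component hit both play the impact emitter and sound before destruction, but only overlaps apply damage.
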(event OnComponentBeginOverlap(Sphere)
  (params (OverlappedComponent :type Primitive%20Component%20Object%20Reference) (OtherActor :type Actor%20Object%20Reference) (OtherComp :type Primitive%20Component%20Object%20Reference) (OtherBodyIndex :type Integer) (bFromSweep :type Boolean) (SweepResult :type Hit%20Result%20Structure%20%28by%20ref%29))
  (bind (_bblockinghit _binitialoverlap _time _distance _location _impactpoint _normal) (Collision|BreakHitResult SweepResult))
  (Utilities|Casting|CastToBP_Unit OtherActor)
  (CallFunction|ApplyDamage OtherActor SweepResult)
  (CallFunction|PlayImpactEffects _impactpoint (Math|Conversions|RotationFromXVector _normal))
  (Actor|DestroyActor))

(event OnComponentHit(Sphere)
  (params (HitComponent :type Primitive%20Component%20Object%20Reference) (OtherActor :type Actor%20Object%20Reference) (OtherComp :type Primitive%20Component%20Object%20Reference) (NormalImpulse :type Vector :default "0, 0, 0") (Hit :type Hit%20Result%20Structure%20%28by%20ref%29))
  (bind _returnvalue (Transformation|GetActorTransform))
  (CallFunction|PlayImpactEffects (.location _returnvalue) (.rotation _returnvalue))
  (Actor|DestroyActor))

(event EventBeginPlay
  (Collision|IgnoreActorwhenMoving (Variables|Default|GetSphere) (Components|GetOwner) true)
  (Collision|SetCollisionEnabled (Variables|Default|GetSphere) "QueryOnly")
  (Actor|SetLifeSpan 1e+01))

(fn ConstructionScript
  (Collision|SetCollisionEnabled (Variables|Default|GetSphere) "NoCollision"))

(fn PlayImpactEffects
  (params (Location :type Vector) (Rotation :type Rotator))
  (Effects|SpawnEmitteratLocation (Variables|Default|GetImpactEffect) Location Rotation)
  (Audio|PlaySoundatLocation (Variables|Default|GetImpactSound) Location "0, 0, 0" 1.0 1.0 0.0 0 0 0 0))

(fn ApplyDamage
  (params (DamagedActor :type Actor%20Object%20Reference) (HitInfo :type Hit%20Result%20Structure%20%28by%20ref%29))
  (Game|Damage|ApplyPointDamage DamagedActor 2e+01 (.TraceStart (Collision|BreakHitResult HitInfo)) HitInfo))