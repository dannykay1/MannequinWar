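; Weapon actor for AI-driven units that fires projectiles at the owner's Blackboard target actor.
; Shortly after BeginPlay it loads damage, fire interval and automatic mode from the unit info DataTable and binds to the owner's BPC_Health killed event.
; FireWeapon shoots once, or repeats on a looping timer when automatic, until StopFiring clears it.
; Each shot spawns a projectile from the muzzle socket with slight random aim scatter, plus muzzle effects.
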(event Custom|Fire
  (bind _returnvalue (Components|GetOwner))
  (bind _target (CallFunction|GetBlackboardTargetActor _returnvalue))
  (Utilities|IsValid _target
    (:Is%20Valid
      (Game|SpawnActorfromClass (Variables|Config|GetProjectileClass) (Math|Transform|MakeTransform (CallFunction|GetMuzzleSocketLocation) (CallFunction|CalculateTargetLookRotation _target) "1.000000,1.000000,1.000000") "Undefined" (Components|GetOwner) (Variables|Default|GetDamage) (Game|GetInstigator))
      (CallFunction|PlayMuzzleEffects))))

(event Custom|FireWeapon
  (Utilities|FlowControl|Sequence
    (:then_0
      (CallFunction|ClearFireTimerHandle))
    (:then_1
      (CallFunction|Fire)
      (if (Variables|Default|GetIsAutomatic?)
        (bind _returnvalue (Utilities|Time|SetTimerbyEvent (delegate Custom|Fire) (Variables|Default|GetTimeBetweenShots) (Variables|Default|GetIsAutomatic?)))
        (Variables|Default|SetFireTimer _returnvalue)))))

(event Custom|StopFiring
  (CallFunction|ClearFireTimerHandle))

(event EventBeginPlay
  (bind _returnvalue (Components|GetOwner))
  (bind _returnvalue_2 (Actor|GetComponentbyClass _returnvalue "/Game/Blueprints/Components/BPC_Health.BPC_Health_C"))
  (Utilities|FlowControl|Delay 0.2)
  (Utilities|FlowControl|Sequence
    (:then_0
      (bind _out_row (Utilities|GetUnitInfoDataTable (Variables|Default|GetRow%20Name))
        (:Row%20Found
          (Variables|Default|SetDamage (.WeaponDamage (Utilities|Struct|BreakST_UnitInfo _out_row)))
          (Variables|Default|SetTimeBetweenShots (.TimeBetweenShots (Utilities|Struct|BreakST_UnitInfo _out_row)))
          (Variables|Default|SetIsAutomatic? (.AutomaticFire? (Utilities|Struct|BreakST_UnitInfo _out_row))))))
    (:then_1
      (Utilities|IsValid _returnvalue_2
        (:Is%20Valid
          (EventDispatchers|BindEventtoOnKilled _returnvalue_2 (EventDispatchers|CreateEvent :!event Custom|StopFiring)))))))

(fn ConstructionScript)

(fn GetMuzzleSocketLocation
  (return (Transformation|GetSocketLocation (Variables|Default|GetWeaponMesh) "Muzzle")))

(fn CalculateTargetLookRotation
  (params (Target :type Actor%20Object%20Reference))
  (return (Math|Rotator|FindLookatRotation (CallFunction|GetMuzzleSocketLocation) (+ (Transformation|GetActorLocation Target) (* (Math|Random|RandomUnitVector) 2e+01)))))

(fn PlayMuzzleEffects
  (Effects|SpawnEmitterAttached (Variables|Config|GetMuzzleEffect) (Variables|Default|GetWeaponMesh) "MuzzleFlash")
  (Audio|SpawnSoundAttached (Variables|Config|GetMuzzleSound) (Variables|Default|GetWeaponMesh) "None" "0, 0, 0" "0, 0, 0" "KeepRelativeOffset" false 1.0 1.0 0.0 0 0))

(fn ClearFireTimerHandle
  (bind _firetimer (Variables|Default|GetFireTimer))
  (if (Utilities|Time|IsValidTimerHandle _firetimer)
    (Utilities|Time|ClearandInvalidateTimerbyHandle _firetimer)))