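; Grenade launcher projectile that bounces with spark and sound effects and explodes on contact.
; Sphere overlaps with actors not on the owner's team, or any sphere hit, trigger a once-only Explode that plays impact effects, applies radial damage ignoring the owner, fires a radial impulse and destroys the actor.
; The first bounce also starts a five-second fuse, which only plays impact effects and destroys the grenade, without damage or impulse.
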(event OnProjectileBounce(ProjectileMovement)
  (params (ImpactResult :type Hit%20Result%20Structure%20%28by%20ref%29) (ImpactVelocity :type Vector%20%28by%20ref%29 :default "0, 0, 0"))
  (Effects|SpawnEmitteratLocation "/Game/MilitaryWeapSilver/FX/P_Impact_Metal_Medium_01.P_Impact_Metal_Medium_01" (Transformation|GetActorLocation))
  (Audio|PlaySoundatLocation "/Game/MilitaryWeapSilver/Sound/GrenadeLauncher/Cues/GrenadeLauncher_Bounce_Cue.GrenadeLauncher_Bounce_Cue" (Transformation|GetActorLocation) "0, 0, 0" 1.0 1.0 0.0 0 0 0 0)
  (Utilities|FlowControl|DoOnce false
    (:Completed
      (Utilities|FlowControl|Delay 5.0)
      (CallFunction|PlayImpactEffects (Transformation|GetActorLocation) "0, 0, 0")
      (Actor|DestroyActor))))

(event OnComponentBeginOverlap(Sphere)
  (params (OverlappedComponent :type Primitive%20Component%20Object%20Reference) (OtherActor :type Actor%20Object%20Reference) (OtherComp :type Primitive%20Component%20Object%20Reference) (OtherBodyIndex :type Integer) (bFromSweep :type Boolean) (SweepResult :type Hit%20Result%20Structure%20%28by%20ref%29))
  (bind (_bblockinghit _binitialoverlap _time _distance _location _impactpoint _normal) (Collision|BreakHitResult SweepResult))
  (Utilities|IsSameTeam? (Components|GetOwner) OtherActor
    (:false
      (CallFunction|Explode _impactpoint (Math|Conversions|RotationFromXVector _normal)))))

(event OnComponentHit(Sphere)
  (params (HitComponent :type Primitive%20Component%20Object%20Reference) (OtherActor :type Actor%20Object%20Reference) (OtherComp :type Primitive%20Component%20Object%20Reference) (NormalImpulse :type Vector :default "0, 0, 0") (Hit :type Hit%20Result%20Structure%20%28by%20ref%29))
  (bind _returnvalue (Transformation|GetActorTransform))
  (CallFunction|Explode (.location _returnvalue) (.rotation _returnvalue)))

(event Custom|Explode
  (params (Location :type Vector) (Rotation :type Rotator))
  (Utilities|FlowControl|DoOnce false
    (:Completed
      (CallFunction|PlayImpactEffects Location Rotation)
      (Game|Damage|ApplyRadialDamage (Variables|Default|GetDamage) (Transformation|GetActorLocation) 5e+02 "/Script/Engine.DamageType" (Utilities|Array|MakeArray (Components|GetOwner)) (Components|GetOwner) (Game|GetInstigatorController) false "ECC_Visibility")
      (Class|RadialForceComponent|FireImpulse (Variables|Default|GetRadialForce))
      (Actor|DestroyActor))))

(event EventBeginPlay
  (|CallParentFunction)
  (Collision|SetCollisionEnabled (Variables|Default|GetSphere) "QueryAndPhysics"))

(event Collision|EventActorBeginOverlap
  (params (OtherActor :type Actor%20Object%20Reference))
  (|CallParentFunction OtherActor) ; This node is disabled and will not be called.\nDrag off pins to build functionality.
)

(event EventTick
  (params (DeltaSeconds :type Float%20%28single-precision%29))
  (|CallParentFunction DeltaSeconds) ; This node is disabled and will not be called.\nDrag off pins to build functionality.
)

(fn ConstructionScript
  (|CallParentFunction))