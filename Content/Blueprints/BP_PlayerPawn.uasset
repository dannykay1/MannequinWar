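; BP_PlayerPawn is a player pawn whose spring-arm camera can be zoomed.
; The Zoom event adds an offset to the current arm length and passes that target to ZoomCamera.
; ZoomCamera plays a timeline that interpolates the spring arm length toward the target each update, clamped between minimum and maximum lengths.
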(event Custom|ZoomCamera
  (params (Amount :type Float%20%28double-precision%29))
  (Timeline|CameraZoom PlayFromStart
    (:Update
      (Variables|/Script/Engine.SpringArmComponent|SetTargetArmLength (Variables|Default|GetSpringArm) (Math|Float|Clamp(Float) (Math|Interpolation|FInterpTo (Variables|/Script/Engine.SpringArmComponent|GetTargetArmLength (Variables|Default|GetSpringArm)) Amount (Utilities|Time|GetWorldDeltaSeconds) 2.5) (Variables|Default|GetMinSpringArmLength) (Variables|Default|GetMaxSpringArmLength))))))

(event EventZoom
  (params (Amount :type Float%20%28double-precision%29))
  (CallFunction|ZoomCamera (+ Amount (Variables|/Script/Engine.SpringArmComponent|GetTargetArmLength (Variables|Default|GetSpringArm)))))

(fn ConstructionScript)